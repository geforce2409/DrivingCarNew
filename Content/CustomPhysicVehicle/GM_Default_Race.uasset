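; Race game mode that spawns and possesses the player's selected car, creates the race HUD and holds all vehicles for three seconds.
; Each Tick scores cars by completed laps plus normalized progress along the track spline, stored in TotalTimes.
; It ranks them by repeatedly taking and clearing the maximum, filling the player/AI standings and lap counter.
; Lap counts are not incremented here, and the off-track teleport logic is disconnected.
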(event `self.ReceiveBeginPlay`
  (bind _returnvalue (`GameplayStatics.GetPlayerController` 0))
  (bind _cars (`self.Cars`))
  (bind _asbp_game_instance (cast `/Game/CustomPhysicVehicle/BP_GameInstance` (`GameplayStatics.GetGameInstance`)))
  (set `self.Number of Laps` (`/Game/CustomPhysicVehicle/BP_GameInstance.Number of Laps` _asbp_game_instance))
  (bind _returnvalue_2 (`|SpawnActorFromClass` (`/Game/CustomPhysicVehicle/BP_GameInstance.Selected Car` _asbp_game_instance) (`self.GetTransform` (`self.K2_FindPlayerStart` null)) "AdjustIfPossibleButAlwaysSpawn" "OverrideRootScale" null true true false true true true true true false true false false false 1.0 1.5 0.5 "/Game/CustomPhysicVehicle/Vehicles/00_Master_Vehicle/Materials/M_default.M_default" "/Game/CustomPhysicVehicle/Vehicles/Camaro/Sounds/Camaro_Engine_Cue.Camaro_Engine_Cue" true null))
  (if (`/Game/CustomPhysicVehicle/Vehicles/00_Master_Vehicle/BP_Master_Vehicle.Is ThirdPerson View` _returnvalue_2)
    (`/Game/CustomPhysicVehicle/Vehicles/00_Master_Vehicle/BP_Master_Vehicle.Change View` _returnvalue_2))
  (set `/Game/CustomPhysicVehicle/Vehicles/00_Master_Vehicle/BP_Master_Vehicle.Can Change View` true _returnvalue_2)
  (set `/Game/CustomPhysicVehicle/Vehicles/00_Master_Vehicle/BP_Master_Vehicle.Mouse for Steering?` false _returnvalue_2)
  (set `/Game/CustomPhysicVehicle/Vehicles/00_Master_Vehicle/BP_Master_Vehicle.Can Display Debug Widget` false _returnvalue_2)
  (set `/Game/CustomPhysicVehicle/Vehicles/00_Master_Vehicle/BP_Master_Vehicle.Anti-Drift Multiplier` 0.5 _returnvalue_2)
  (`Controller.Possess` _returnvalue _returnvalue_2)
  (bind _returnvalue_3 (`|CreateWidget` "/Game/CustomPhysicVehicle/UMG/UMG_Race.UMG_Race_C" _returnvalue))
  (set `self.HUD` _returnvalue_3)
  (`UserWidget.AddToViewport` _returnvalue_3 0)
  (bind _outactors (`GameplayStatics.GetAllActorsWithTag` "Race"))
  (bind _asbp_track_spline (cast `/Game/CustomPhysicVehicle/Environment/RaceTrack/BP_Track_Spline` (`|GetArrayItem` _outactors)))
  (set `self.Track` _asbp_track_spline)
  (bind _outactors_2 (`GameplayStatics.GetAllActorsOfClass` "/Game/CustomPhysicVehicle/Vehicles/00_Master_Vehicle/BP_Master_Vehicle.BP_Master_Vehicle_C"))
  (for _array_element _outactors_2
    (`KismetArrayLibrary.Array_Add` _cars _array_element)
    (`/Game/CustomPhysicVehicle/Vehicles/00_Master_Vehicle/BP_Master_Vehicle.Server_Handbrake` _array_element true)
    (`self.DisableInput` _array_element null)
    (`KismetArrayLibrary.Array_Add` (`self.Laps`))
    (`KismetArrayLibrary.Array_Add` (`self.Total Times`))
    (`KismetArrayLibrary.Array_Add` (`self.Best Lap Time`))
    (bind _returnvalue_4 (`|CreateWidget` "/Game/CustomPhysicVehicle/UMG/Text.Text_C"))
    (`VerticalBox.AddChildToVerticalBox` (`/Game/CustomPhysicVehicle/UMG/UMG_Race.CarList` (`self.HUD`)) _returnvalue_4)
    (bind _asbp_controller (cast `/Game/CustomPhysicVehicle/BP_Controller` (`Pawn.GetController` _array_element)))
    (`/Game/CustomPhysicVehicle/BP_Controller.Show Vehicle HUD` _asbp_controller))
  (`KismetSystemLibrary.Delay` 3.0)
  (for _array_element_2 _cars
    (`/Game/CustomPhysicVehicle/Vehicles/00_Master_Vehicle/BP_Master_Vehicle.Server_Handbrake` _array_element_2 false)
    (`self.EnableInput` _array_element_2 null)
    (if (`/Game/CustomPhysicVehicle/Vehicles/00_Master_Vehicle/BP_Master_Vehicle.Is Player Controlled` _array_element_2)
      _
      (else
        _))
    (`KismetArrayLibrary.Array_Add` (`self.Lap Start Time`) (`KismetSystemLibrary.GetGameTimeInSeconds`))))

(event `self.ReceiveTick`
  (params (DeltaSeconds :type "Float (single-precision)"))
  (bind _total_times (`self.Total Times`))
  (bind _indexofmaxvalue (`KismetMathLibrary.MaxOfFloatArray` _total_times))
  (bind _spline (`/Game/CustomPhysicVehicle/Environment/RaceTrack/BP_Track_Spline.Spline` (`self.Track`)))
  (bind _returnvalue (`Pawn.GetController` (`|GetArrayItem` (`self.Cars`) _indexofmaxvalue)))
  (for (_array_element _array_index) (`self.Cars`)
    (`KismetArrayLibrary.Array_Set` (`self.Total Times`) _array_index (+ (/ (`SplineComponent.FindInputKeyClosestToWorldLocation` _spline (`SplineComponent.FindLocationClosestToWorldLocation` _spline (`self.K2_GetActorLocation` _array_element) "World")) (`KismetMathLibrary.Conv_IntToDouble` (`SplineComponent.GetNumberOfSplinePoints` _spline))) (`KismetMathLibrary.Conv_IntToDouble` (`|GetArrayItem` (`self.Laps`) _array_index)))))
  (for (_ _array_index_2) (`self.Cars`)
    (`/Engine/EditorBlueprintResources/StandardMacros.IsValid` _returnvalue
      (:`Is Valid`
        (bind _astext (cast `/Game/CustomPhysicVehicle/UMG/Text` (`PanelWidget.GetChildAt` (`/Game/CustomPhysicVehicle/UMG/UMG_Race.CarList` (`self.HUD`)) _array_index_2)))
        (bind _asbp_ai_race (cast `/Game/CustomPhysicVehicle/Vehicles/01_AI/BP_AI_Race` _returnvalue)
          (:`then`
            (bind _text (`/Game/CustomPhysicVehicle/UMG/Text.Text` _astext))
            (`TextBlock.SetText` _text (`KismetTextLibrary.Conv_StringToText` (`KismetStringLibrary.Concat_StrStr` (`KismetStringLibrary.Conv_IntToString` (+ _array_index_2 1)) ". " (`KismetTextLibrary.Conv_TextToString` (`/Game/CustomPhysicVehicle/Vehicles/01_AI/BP_AI_Race.Name` _asbp_ai_race)))))
            (`TextBlock.SetColorAndOpacity` _text (make `SlateColor` (struct :`R` 1.0 :`G` 1.0 :`B` 1.0 :`A` 1.0))))
          (:`CastFailed`
            (bind _text_2 (`/Game/CustomPhysicVehicle/UMG/Text.Text` _astext))
            (`TextBlock.SetText` _text_2 (`KismetTextLibrary.Conv_StringToText` (`KismetStringLibrary.Concat_StrStr` (`KismetStringLibrary.Conv_IntToString` (+ _array_index_2 1)) ". " "Player")))
            (`TextBlock.SetColorAndOpacity` _text_2 (make `SlateColor` (struct :`R` 0.031586 :`G` 0.255208 :`A` 1.0)))))
        (`KismetArrayLibrary.Array_Set` _total_times _indexofmaxvalue))))
  (for (_array_element_2 _array_index_3) (`self.Cars`)
    (if (`Pawn.IsPlayerControlled` _array_element_2)
      (`TextBlock.SetText` (`/Game/CustomPhysicVehicle/UMG/UMG_Race.Laps` (`self.HUD`)) (`KismetTextLibrary.Conv_StringToText` (`KismetStringLibrary.Concat_StrStr` (`KismetStringLibrary.Conv_IntToString` (`|GetArrayItem` (`self.Laps`) _array_index_3)) "/" (`KismetStringLibrary.Conv_IntToString` (`self.Number of Laps`))))))))

(fn `UserConstructionScript`)