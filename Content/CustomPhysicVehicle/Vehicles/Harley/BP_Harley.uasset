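; Drivable physics-based Harley motorcycle pawn with a visible rider who ragdolls off in crashes.
; Throttle drives the rear-wheel constraint through simulated RPM and speed-based automatic two-gear shifting, while steering turns the fork constraint, damped by speed.
; Each tick, an interpolated center-of-mass offset from roll, steering and speed balances the bike, with angular velocity zeroed.
; Hard hits or excessive tilt eject the rider; Interact then possesses a new BP_Physic_Pawn spawned there.
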(event `self.ReceivePossessed`
  (params (NewController :type "Controller Object Reference"))
  (if (`Controller.IsPlayerController` NewController)
    (`SceneComponent.SetVisibility` (`self.Driver`) true false)
    (`self.Player_Reset`)
    (bind _asharley_rider_anim_bp (cast `/Game/CustomPhysicVehicle/Vehicles/Harley/Harley_Rider_AnimBP` (`SkeletalMeshComponent.GetAnimInstance` (`self.Driver`))))
    (set `self.Rider AnimBP` _asharley_rider_anim_bp)))

(event `self.ReceiveUnpossessed`
  (params (OldController :type "Controller Object Reference"))
  (`SceneComponent.SetVisibility` (`self.Driver`) false false))

(event `self.ReceiveTick`
  (params (DeltaSeconds :type "Float (single-precision)"))
  (bind _rider_animbp (`self.Rider AnimBP`))
  (bind _returnvalue (* (`KismetMathLibrary.VSize` (`SceneComponent.GetComponentVelocity` (`self.Mesh`))) 0.036))
  (if (`self.IsControlled`)
    _
    (else
      _))
  (`self.Look Around`)
  (`self.Balance Forces`)
  (`/Engine/EditorBlueprintResources/StandardMacros.IsValid` _rider_animbp
    (:`Is Valid`
      (set `/Game/CustomPhysicVehicle/Vehicles/Harley/Harley_Rider_AnimBP.Speed` (* (`KismetMathLibrary.VSize` (`SceneComponent.GetComponentVelocity` (`self.Mesh`))) 0.036) _rider_animbp))
    (:`Is Not Valid`
      _))
  (if (and (> _returnvalue 40.0) (== (`self.Gear`) 0))
    (set `self.Gear` 1)
    (set `self.Is Changing Gear` true :!label _label)
    (`KismetSystemLibrary.Delay` 0.5)
    (set `self.Is Changing Gear` false)
    (elif (and (> 30.0 _returnvalue) (== (`self.Gear`) 1))
      (set `self.Gear` 0)
      (goto _label))))

(event `InputAxis|MoveRight`
  (params (AxisValue :type "Float (single-precision)"))
  (if (and (`self.IsControlled`) (not (`self.Player Ejected`)))
    (`self.Set Steering` AxisValue)
    (else
      (`self.Set Steering` 0.0))))

(event `InputAxis|MoveForward`
  (params (AxisValue :type "Float (single-precision)"))
  (if (and (`self.IsControlled`) (not (`self.Player Ejected`)))
    (`self.Set Throttle` AxisValue)
    (else
      (`self.Set Throttle` 0.0))))

(event `Player_Reset`
  (bind _mesh (`self.Mesh`))
  (bind _driver (`self.Driver`))
  (bind (_returnvalue_roll _returnvalue_pitch _returnvalue_yaw) (`KismetMathLibrary.BreakRotator` (`SceneComponent.K2_GetComponentRotation` _mesh)))
  (`SceneComponent.K2_SetWorldRotation` _mesh (`KismetMathLibrary.MakeRotator` 0.0 0.0 _returnvalue_yaw) false true)
  (set `self.Player Ejected` false)
  (`PrimitiveComponent.SetCollisionEnabled` _driver "NoCollision" :!label _label_2)
  (`PrimitiveComponent.SetSimulatePhysics` _driver false)
  (`SceneComponent.K2_AttachToComponent` _driver (`self.Mesh`) "None" "SnapToTarget" "SnapToTarget" "SnapToTarget" false)
  (`SceneComponent.K2_SetRelativeTransform` _driver (`KismetMathLibrary.MakeTransform` (0.0 -1.829569 -0.115044)) false true))

(event `InputAction|Interact`
  (params (Key :type "Key Structure"))
  (bind _returnvalue (`SceneComponent.K2_GetComponentToWorld` (`self.Driver`)))
  (:`Pressed`
    (if (`self.Player Ejected`)
      (bind _returnvalue_2 (`|SpawnActorFromClass` "/Game/CustomPhysicVehicle/Player/BP_Physic_Pawn.BP_Physic_Pawn_C" (`KismetMathLibrary.MakeTransform` (+ (.location _returnvalue) (0.0 0.0 100.0)) (`KismetMathLibrary.MakeRotator` 0.0 0.0 (.yaw (.rotation _returnvalue)))) "AdjustIfPossibleButAlwaysSpawn" "OverrideRootScale" null true null))
      (set `/Game/CustomPhysicVehicle/Player/BP_Physic_Pawn.Camera Rot` (`self.GetControlRotation`) _returnvalue_2)
      (`Controller.Possess` (`self.GetController`) _returnvalue_2)
      (goto _label_2))))

(event `self.Mesh.OnComponentHit`
  (params (HitComponent :type "PrimitiveComponent Object Reference") (OtherActor :type "Actor Object Reference") (OtherComp :type "PrimitiveComponent Object Reference") (NormalImpulse :type "Vector Structure") (Hit :type "HitResult Structure (by ref)"))
  (bind _x (.x NormalImpulse))
  (bind _y (.y NormalImpulse))
  (if (and (`self.IsControlled`) (not (`self.Player Ejected`)))
    (if (> (`KismetMathLibrary.VSize` (`KismetMathLibrary.MakeVector` _x _y)) 11500.0)
      (`self.Driver Eject`)
      (`PrimitiveComponent.AddImpulse` (`self.Driver`) (`KismetMathLibrary.MakeVector` (* _x -0.0075) (* _y -0.0075)) "spine_02" true))))

(fn `Balance Forces`
  (bind _returnvalue (`KismetMathLibrary.FInterpTo` (`self.COM Offset`) (+ (`KismetMathLibrary.MapRangeClamped` (.roll (`SceneComponent.RelativeRotation` (`self.Mesh`))) -50.0 50.0 250.0 -250.0) (* (`KismetMathLibrary.MapRangeClamped` (`self.Steering`) -1.0 1.0 -85.0 85.0) (`KismetMathLibrary.MapRangeClamped` (* (`KismetMathLibrary.VSize` (`SceneComponent.GetComponentVelocity` (`self.Mesh`))) 0.036) 0.0 100.0 0.0 3.0))) (`GameplayStatics.GetWorldDeltaSeconds`) 20.0))
  (if (`self.Player Ejected`)
    (`PrimitiveComponent.SetCenterOfMass` (`self.Mesh`) (0.0 0.0 0.0) "None")
    (else
      (`PrimitiveComponent.SetCenterOfMass` (`self.Mesh`) (`KismetMathLibrary.MakeVector` 0.0 _returnvalue 40.0) "None")
      (set `self.COM Offset` _returnvalue)
      (`PrimitiveComponent.SetPhysicsAngularVelocityInDegrees` (`self.Mesh`) (0.0 0.0 0.0) false "None")
      (if (and (`KismetMathLibrary.InRange_FloatFloat` (.roll (`SceneComponent.RelativeRotation` (`self.Mesh`))) -65.0 65.0) (`KismetMathLibrary.InRange_FloatFloat` (.pitch (`SceneComponent.RelativeRotation` (`self.Mesh`))) -10.0 40.0))
        _
        (elif (not (`self.Player Ejected`))
          (`self.Driver Eject`)))))
  (return))

(fn `Driver Eject`
  (bind _driver (`self.Driver`))
  (if (not (`self.Player Ejected`))
    (set `self.Player Ejected` true)
    (`SceneComponent.K2_DetachFromComponent` _driver "KeepWorld" "KeepWorld" "KeepWorld" true)
    (`PrimitiveComponent.SetSimulatePhysics` _driver true)
    (`PrimitiveComponent.SetCollisionObjectType` _driver "ECC_PhysicsBody")
    (`PrimitiveComponent.SetCollisionEnabled` _driver "QueryAndPhysics")))

(fn `Look Around`
  (`self.AddControllerPitchInput` (* (`self.GetInputAxisValue`) -1.0))
  (`self.AddControllerYawInput` (`self.GetInputAxisValue`)))

(fn `Set Steering`
  (params (`Axis Value` :type "Float (double-precision)"))
  (bind _output_get (set `self.Steering` `Axis Value`))
  (`PhysicsConstraintComponent.SetAngularOrientationTarget` (`self.PC_Fork`) (`KismetMathLibrary.MakeRotator` 0.0 0.0 (* _output_get -25.0 (`KismetMathLibrary.MapRangeClamped` (* (`KismetMathLibrary.VSize` (`SceneComponent.GetComponentVelocity` (`self.Mesh`))) 0.036) 0.0 50.0 1.0 0.2)))))

(fn `Set Throttle`
  (params (`Axis Value` :type "Float (double-precision)"))
  (bind _rpm_limiter (`self.RPM Limiter`))
  (if (`self.Engine Started`)
    (if (and (> `Axis Value` 0.0) (not (`self.Is Changing Gear`)))
      (if (<= (`self.RPM`) _rpm_limiter)
        (set `self.Is Accelerating` true)
        (set `self.RPM` (+ (`self.RPM`) (* (* (`KismetMathLibrary.Sqrt` (`self.RPM_Rise`)) (`KismetMathLibrary.Abs` `Axis Value`)) (`GameplayStatics.GetWorldDeltaSeconds`))))
        (`PhysicsConstraintComponent.SetAngularVelocityTarget` (`self.PC_Rear`) (`KismetMathLibrary.MakeVector` 0.0 (/ (/ (/ (`self.RPM Max`) (* (`.GearRatio_45_10E21ADD448930CC200DADBAFC7B8AC3` (break `/Game/CustomPhysicVehicle/Vehicles/00_Master_Vehicle/Structs/Gear_Structure` (`|GetArrayItem` (`self.Gears`) (`self.Gear`)))) (`self.Differential Ratio`))) 3.6) 37.648083)))
        (`PhysicsConstraintComponent.SetAngularDriveParams` (`self.PC_Rear`) 0.0 (* (`self.Engine Torque`) (`self.RPM`) (* (`.GearRatio_45_10E21ADD448930CC200DADBAFC7B8AC3` (break `/Game/CustomPhysicVehicle/Vehicles/00_Master_Vehicle/Structs/Gear_Structure` (`|GetArrayItem` (`self.Gears`) (`self.Gear`)))) (`self.Differential Ratio`))) 0.0)
        (else
          (set `self.RPM` (- _rpm_limiter 500.0))
          (`PhysicsConstraintComponent.SetAngularDriveParams` (`self.PC_Rear`) 0.0 0.0 0.0 :!label _label)))
      (elif (>= (`self.RPM`) (select `bool` (`self.Engine Started`) :`true` (`self.RPM Idle`)))
        (set `self.Is Accelerating` false)
        (set `self.RPM` (- (`self.RPM`) (* (* (`self.RPM Fall`) (`KismetMathLibrary.SelectFloat` 0.0 1.0 (`self.Is Changing Gear`))) (`GameplayStatics.GetWorldDeltaSeconds`))))
        (goto _label)
        (else
          (goto _label))))))

(fn `UserConstructionScript`)