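; Game mode for free roam that puts the player in a drivable Camaro when play begins.
; It spawns BP_Camaro at a player start with default paint and engine sound, turns off camera auto-rotation and has the first player controller possess it.
; It then shows the vehicle HUD through the BP_Controller of the master vehicles in the level.
; The car class is hard-coded, as the game instance's SelectedCar is unused.
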(event `self.ReceiveBeginPlay`
  (bind _asbp_game_instance (cast `/Game/CustomPhysicVehicle/BP_GameInstance` (`GameplayStatics.GetGameInstance`)))
  (bind _returnvalue (`|SpawnActorFromClass` "/Game/CustomPhysicVehicle/Vehicles/Camaro/BP_Camaro.BP_Camaro_C" (`self.GetTransform` (`self.K2_FindPlayerStart` null)) "AdjustIfPossibleButAlwaysSpawn" "OverrideRootScale" null true true true true true true false true false true true false false 1.0 0.9 0.3 "/Game/CustomPhysicVehicle/Vehicles/00_Master_Vehicle/Materials/M_default.M_default" "/Game/CustomPhysicVehicle/Vehicles/Camaro/Sounds/Camaro_Engine_Cue.Camaro_Engine_Cue" true null))
  (set `/Game/CustomPhysicVehicle/Vehicles/00_Master_Vehicle/BP_Master_Vehicle.Auto Rotate Camera` false _returnvalue)
  (`Controller.Possess` (`GameplayStatics.GetPlayerController` 0) _returnvalue)
  (bind _outactors (`GameplayStatics.GetAllActorsOfClass` "/Game/CustomPhysicVehicle/Vehicles/00_Master_Vehicle/BP_Master_Vehicle.BP_Master_Vehicle_C"))
  (for _array_element _outactors
    (bind _asbp_controller (cast `/Game/CustomPhysicVehicle/BP_Controller` (`Pawn.GetController` _array_element)))
    (`/Game/CustomPhysicVehicle/BP_Controller.Show Vehicle HUD` _asbp_controller)))

(fn `UserConstructionScript`)