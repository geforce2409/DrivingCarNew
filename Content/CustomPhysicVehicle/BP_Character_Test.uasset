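; Test character that reacts to being struck by moving objects, apparently for custom physics vehicle testing.
; Capsule hits launch the character along the hit normal, scaled by the other actor's speed.
; Vehicle_Detect overlaps above a speed threshold switch the capsule to query-only, enable mesh physics for a ragdoll, and apply a speed-scaled impulse at the sweep location.
; An alternative launch on overlap is left unconnected.
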(event `self.CapsuleComponent.OnComponentHit`
  (params (HitComponent :type "PrimitiveComponent Object Reference") (OtherActor :type "Actor Object Reference") (OtherComp :type "PrimitiveComponent Object Reference") (NormalImpulse :type "Vector Structure") (Hit :type "HitResult Structure (by ref)"))
  (`self.LaunchCharacter` (* (`.Normal` (`GameplayStatics.BreakHitResult` Hit)) (* (`KismetMathLibrary.VSize` (`self.GetVelocity` OtherActor)) 1.0 5.0))))

(event `self.Vehicle_Detect.OnComponentBeginOverlap`
  (params (OverlappedComponent :type "PrimitiveComponent Object Reference") (OtherActor :type "Actor Object Reference") (OtherComp :type "PrimitiveComponent Object Reference") (OtherBodyIndex :type Integer) (bFromSweep :type Boolean) (SweepResult :type "HitResult Structure (by ref)"))
  (bind (_bblockinghit _binitialoverlap _time _distance _location _impactpoint _normal) (`GameplayStatics.BreakHitResult` SweepResult))
  (bind _mesh (`self.Mesh`))
  (bind _returnvalue (`KismetMathLibrary.VSize` (`SceneComponent.GetComponentVelocity` OtherComp)))
  (if (> _returnvalue 350.0)
    (`PrimitiveComponent.SetCollisionEnabled` (`self.CapsuleComponent`) "QueryOnly")
    (`PrimitiveComponent.SetSimulatePhysics` _mesh true)
    (`PrimitiveComponent.AddImpulseAtLocation` _mesh (* _normal (* _returnvalue 1.0 10000.0)) _location "None")))

(fn `UserConstructionScript`)