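; Environment actor that sets up the sky sphere, directional sun and sky light from exposed color, brightness, cloud and angle properties.
; The construction script creates a dynamic panning-cloud sky material and applies each property through small setter functions.
; Sun rotation and color feed back into the material's light direction, sun height and sun color before the sky light recaptures.
; No runtime time-of-day logic is present, as OnRep_Time is empty.
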(fn `OnRep_Time`)

(fn `UserConstructionScript`
  (bind _sun_light_color (`self.Sun Light Color`))
  (bind _overall_color (`self.Overall Color`))
  (bind _returnvalue (`KismetMathLibrary.MapRangeUnclamped` (.pitch (`SceneComponent.K2_GetComponentRotation` (`self.Sun_Light`))) 0.0 -90.0 0.0 1.0))
  (bind _returnvalue_2 (`PrimitiveComponent.CreateDynamicMaterialInstance` (`self.Sky Sphere mesh`) 0 "/Engine/EngineSky/M_Sky_Panning_Clouds2.M_Sky_Panning_Clouds2" "None"))
  (set `self.Sky material` _returnvalue_2)
  (`MaterialInstanceDynamic.SetScalarParameterValue` (`self.Sky material`) "Cloud speed" (`self.Cloud speed`))
  (`MaterialInstanceDynamic.SetScalarParameterValue` (`self.Sky material`) "Stars Brightness" (`self.Stars brightness`))
  (`MaterialInstanceDynamic.SetScalarParameterValue` (`self.Sky material`) "Sun brightness" (`self.Sun brightness`))
  (`MaterialInstanceDynamic.SetScalarParameterValue` (`self.Sky material`) "Sun Radius" (`self.Sun Radius`))
  (`SceneComponent.K2_SetWorldRotation` (`self.Sun_Light`) (`KismetMathLibrary.MakeRotator` 0.0 (`self.Sun Pitch Angle`) (`self.Sun Yaw Angle`)) false false)
  (`SkyLightComponent.SetIntensity` (`self.Sky_Light`) (`self.Sky Light Intensity`))
  (`LightComponent.SetIntensity` (`self.Sun_Light`) (`self.Sun Light Intensity`))
  (`MaterialInstanceDynamic.SetScalarParameterValue` (`self.Sky material`) "Cloud Opacity" (`self.Cloud Opacity`))
  (`MaterialInstanceDynamic.SetScalarParameterValue` (`self.Sky material`) "Horizon falloff" (`self.Horizon Falloff`))
  (`MaterialInstanceDynamic.SetVectorParameterValue` (`self.Sky material`) "Horizon color" (`self.Horizon Color`))
  (`LightComponent.SetLightColor` (`self.Sun_Light`) _sun_light_color true)
  (`LightComponent.SetBloomTint` (`self.Sun_Light`) (`KismetMathLibrary.Conv_LinearColorToColor` _sun_light_color))
  (`MaterialInstanceDynamic.SetVectorParameterValue` (`self.Sky material`) "Zenith color" (`self.Zenith Color`))
  (`MaterialInstanceDynamic.SetVectorParameterValue` (`self.Sky material`) "Overall color" _overall_color)
  (`SkyLightComponent.SetLightColor` (`self.Sky_Light`) _overall_color)
  (`MaterialInstanceDynamic.SetVectorParameterValue` (`self.Sky material`) "Cloud color" (`self.Cloud Color`))
  (`MaterialInstanceDynamic.SetVectorParameterValue` (`self.Sky material`) "Light direction" (`KismetMathLibrary.Conv_VectorToLinearColor` (`KismetMathLibrary.Conv_RotatorToVector` (`SceneComponent.K2_GetComponentRotation` (`self.Sun_Light`)))))
  (`MaterialInstanceDynamic.SetScalarParameterValue` (`self.Sky material`) "Sun height" (`KismetMathLibrary.SelectFloat` (`KismetMathLibrary.Abs` _returnvalue) 0.0 (< _returnvalue 0.0)))
  (`MaterialInstanceDynamic.SetVectorParameterValue` (`self.Sky material`) "Sun color" (`LightComponentBase.GetLightColor` (`self.Sun_Light`)))
  (`SkyLightComponent.RecaptureSky` (`self.Sky_Light`)))