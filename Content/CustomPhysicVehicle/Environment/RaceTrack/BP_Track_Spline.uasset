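; Race track actor that builds a road from spline meshes along an optionally looped spline.
; Construction script splits the spline into NumberOfMeshes equal segments with matched tangents and roll, taking each mesh from the Struct array and appending default Track entries where missing.
; Each segment gets an index text label, and the UpdateLandscape one-shot toggle deforms the first Landscape to the spline.
; Helper functions compute per-point offset endpoints and roll, but construction never calls them.
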(fn `Track Roll`
  (params (PointIndex :type Integer))
  (returns (`Start Roll` :type "Float (double-precision)") (`End Roll` :type "Float (double-precision)") (`Any Roll?` :type Boolean))
  (bind _spline (`self.Spline`))
  (bind _returnvalue (`SplineComponent.GetRollAtSplinePoint` _spline (+ PointIndex 1) "Local"))
  (bind _returnvalue_2 (`SplineComponent.GetRollAtSplinePoint` _spline PointIndex "Local"))
  (return (/ _returnvalue_2 25.0) (/ _returnvalue 25.0) (or (> (`KismetMathLibrary.Abs` _returnvalue_2) 1.0) (> (`KismetMathLibrary.Abs` _returnvalue) 1.0))))

(fn `Track Start-End`
  (params (`Lateral Offset` :type "Float (double-precision)") (PointIndex :type Integer))
  (returns (`Start Tangent` :type "Vector Structure") (`Start Location` :type "Vector Structure") (`End Tangent` :type "Vector Structure") (`End Location` :type "Vector Structure"))
  (bind _returnvalue (+ PointIndex 1))
  (bind _spline (`self.Spline`))
  (bind (_returnvalue_location _returnvalue_rotation) (`KismetMathLibrary.BreakTransform` (`SplineComponent.GetTransformAtSplinePoint` _spline PointIndex "Local" false)))
  (bind _returnvalue_2 (`KismetMathLibrary.SelectInt` _returnvalue (`KismetMathLibrary.SelectInt` 0 PointIndex (`self.Connect Last to First`)) (<= _returnvalue (- (`SplineComponent.GetNumberOfSplinePoints` (`self.Spline`)) 1))))
  (bind (_returnvalue_location_2 _returnvalue_rotation_2) (`KismetMathLibrary.BreakTransform` (`SplineComponent.GetTransformAtSplinePoint` _spline _returnvalue_2 "Local" false)))
  (return (`SplineComponent.GetTangentAtSplinePoint` _spline PointIndex "Local") (+ (+ _returnvalue_location (* (`KismetMathLibrary.GetRightVector` _returnvalue_rotation) `Lateral Offset`)) (0.0 0.0 10.0) (* (`KismetMathLibrary.GetForwardVector` _returnvalue_rotation) 0.0)) (`SplineComponent.GetTangentAtSplinePoint` _spline _returnvalue_2 "Local") (+ (+ _returnvalue_location_2 (* (`KismetMathLibrary.GetRightVector` _returnvalue_rotation_2) `Lateral Offset`)) (0.0 0.0 10.0) (* (`KismetMathLibrary.GetForwardVector` _returnvalue_rotation_2) 0.0))))

(fn `UserConstructionScript`
  (bind _struct (`self.Struct`))
  (bind _index (`self.Index`))
  (bind _returnvalue (* (`self.Index`) (`self.Length per Mesh`)))
  (bind _output_mesh (break `/Game/CustomPhysicVehicle/Environment/RaceTrack/Track_Struct` (`|GetArrayItem` _struct _index)))
  (bind _returnvalue_2 (* (+ (`self.Index`) 1) (`self.Length per Mesh`)))
  (bind _returnvalue_3 (`SplineComponent.GetTransformAtDistanceAlongSpline` (`self.Spline`) (* (+ (`self.Index`) 1) (`self.Length per Mesh`)) "Local" true))
  (bind _returnvalue_4 (/ (+ 0.0 (.yaw (.rotation _returnvalue_3))) 1.0))
  (bind _returnvalue_5 (/ (+ 0.0 (.roll (.rotation _returnvalue_3))) 1.0))
  (bind _returnvalue_6 (/ (+ 0.0 (.pitch (.rotation _returnvalue_3))) 1.0))
  (`SplineComponent.SetClosedLoop` (`self.Spline`) (`self.Connect Last to First`) true)
  (set `self.Length per Mesh` (/ (`SplineComponent.GetSplineLength` (`self.Spline`)) (`KismetMathLibrary.Conv_IntToDouble` (`self.Number of Meshes`))))
  (for _index_2 (range (`self.Number of Meshes`))
    (set `self.Index` _index_2)
    (bind _returnvalue_7 (`AddComponent|NODE_AddSplineMeshComponent-7`))
    (`SplineMeshComponent.SetStartAndEnd` _returnvalue_7 (`SplineComponent.GetLocationAtDistanceAlongSpline` (`self.Spline`) _returnvalue "Local") (* (`KismetMathLibrary.Normal` (`SplineComponent.GetTangentAtDistanceAlongSpline` (`self.Spline`) _returnvalue "Local")) (`self.Length per Mesh`)) (`SplineComponent.GetLocationAtDistanceAlongSpline` (`self.Spline`) _returnvalue_2 "Local") (* (`KismetMathLibrary.Normal` (`SplineComponent.GetTangentAtDistanceAlongSpline` (`self.Spline`) _returnvalue_2 "Local")) (`self.Length per Mesh`)) true)
    (`SplineMeshComponent.SetStartRoll` _returnvalue_7 (/ (`SplineComponent.GetRollAtDistanceAlongSpline` (`self.Spline`) (* (`self.Index`) (`self.Length per Mesh`)) "Local") 90.0) true)
    (`SplineMeshComponent.SetEndRoll` _returnvalue_7 (/ (`SplineComponent.GetRollAtDistanceAlongSpline` (`self.Spline`) (* (+ (`self.Index`) 1) (`self.Length per Mesh`)) "Local") 90.0) true)
    (if (`KismetArrayLibrary.Array_IsValidIndex` (`self.Struct`) _index)
      (`StaticMeshComponent.SetStaticMesh` _returnvalue_7 _output_mesh)
      (else
        (`KismetArrayLibrary.Array_Add` _struct (make `/Game/CustomPhysicVehicle/Environment/RaceTrack/Track_Struct` "/Game/CustomPhysicVehicle/Environment/RaceTrack/Track.Track"))))
    (bind _returnvalue_8 (`AddComponent|NODE_AddTextRenderComponent-1` :`RelativeTransform` (`KismetMathLibrary.MakeTransform` (+ (/ (+ (.location (`SplineComponent.GetTransformAtDistanceAlongSpline` (`self.Spline`) (* (`self.Index`) (`self.Length per Mesh`)) "Local" true)) (.location _returnvalue_3)) 2.0) (0.0 0.0 100.0) (* (`KismetMathLibrary.GetForwardVector` (`KismetMathLibrary.MakeRotator` _returnvalue_5 _returnvalue_6 (+ _returnvalue_4 90.0))) 700.0)) (`KismetMathLibrary.MakeRotator` (+ _returnvalue_5 0.0) (+ _returnvalue_6 75.0) (+ _returnvalue_4 180.0)) (5.0 5.0 5.0))))
    (`TextRenderComponent.K2_SetText` _returnvalue_8 (`KismetTextLibrary.Conv_IntToText` (`self.Index`)))
    (if (`self.Update Landscape`)
      (set `self.Update Landscape` false)
      (bind _outactors (`GameplayStatics.GetAllActorsOfClass` "/Script/Landscape.Landscape"))
      (`LandscapeProxy.EditorApplySpline` (`|GetArrayItem` _outactors) (`self.Spline`) 900.0 900.0 2000.0 2000.0 0.0 0.0 20 true true null))))