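; Finish line trigger for the race track that counts laps and times them for each BP_Master_Vehicle.
; When a component tagged VehicleMesh overlaps the box, it updates per-car lap count, start time and best time arrays in GM_Default_Race.
; The first crossing starts timing without recording a best lap.
; For player-controlled cars, it also writes the formatted best lap to the game mode's HUD.
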(event `self.Box.OnComponentBeginOverlap`
  (params (OverlappedComponent :type "PrimitiveComponent Object Reference") (OtherActor :type "Actor Object Reference") (OtherComp :type "PrimitiveComponent Object Reference") (OtherBodyIndex :type Integer) (bFromSweep :type Boolean) (SweepResult :type "HitResult Structure (by ref)"))
  (if (`KismetArrayLibrary.Array_Contains` (`ActorComponent.ComponentTags` OtherComp) "VehicleMesh")
    (bind _asbp_master_vehicle (cast `/Game/CustomPhysicVehicle/Vehicles/00_Master_Vehicle/BP_Master_Vehicle` OtherActor))
    (bind _laps (`/Game/CustomPhysicVehicle/GM_Default_Race.Laps` (stale `self.ReceiveBeginPlay` _asgm_default_race)))
    (bind _cars (`/Game/CustomPhysicVehicle/GM_Default_Race.Cars` (stale `self.ReceiveBeginPlay` _asgm_default_race)))
    (bind _returnvalue (`KismetArrayLibrary.Array_Find` _cars _asbp_master_vehicle))
    (bind _output (`|GetArrayItem` _laps _returnvalue))
    (`KismetArrayLibrary.Array_Set` _laps _returnvalue (+ _output 1))
    (bind _lap_start_time (`/Game/CustomPhysicVehicle/GM_Default_Race.Lap Start Time` (stale `self.ReceiveBeginPlay` _asgm_default_race)))
    (bind _returnvalue_2 (- (`KismetSystemLibrary.GetGameTimeInSeconds`) (`|GetArrayItem` _lap_start_time _returnvalue)))
    (bind _best_lap_time (`/Game/CustomPhysicVehicle/GM_Default_Race.Best Lap Time` (stale `self.ReceiveBeginPlay` _asgm_default_race)))
    (bind _output_2 (`|GetArrayItem` _best_lap_time _returnvalue))
    (if (< _returnvalue_2 _output_2)
      (if (not (== _output 1))
        (`KismetArrayLibrary.Array_Set` _best_lap_time _returnvalue _returnvalue_2 true))
      (`KismetArrayLibrary.Array_Set` _lap_start_time _returnvalue (`KismetSystemLibrary.GetGameTimeInSeconds`) true :!label _label)
      (if (`Pawn.IsPlayerControlled` (`|GetArrayItem` _cars _returnvalue))
        (bind _asgm_default_race (cast `/Game/CustomPhysicVehicle/GM_Default_Race` (`GameplayStatics.GetGameMode`)))
        (bind (_days _hours _minutes _seconds _milliseconds) (`KismetMathLibrary.BreakTimespan` (`KismetMathLibrary.FromSeconds` _output_2)))
        (`TextBlock.SetText` (`/Game/CustomPhysicVehicle/UMG/UMG_Race.Best_Lap` (`/Game/CustomPhysicVehicle/GM_Default_Race.HUD` _asgm_default_race)) (`KismetTextLibrary.Conv_StringToText` (`KismetStringLibrary.Concat_StrStr` (`KismetStringLibrary.Concat_StrStr` (`KismetMathLibrary.SelectString` "0" "" (< _minutes 10)) (`KismetStringLibrary.Conv_IntToString` _minutes)) ":" (`KismetStringLibrary.Concat_StrStr` (`KismetMathLibrary.SelectString` "0" "" (< _seconds 10)) (`KismetStringLibrary.Conv_IntToString` _seconds)) "." (`KismetStringLibrary.Conv_IntToString` _milliseconds)))))
      (elif (== _output 1)
        (`KismetArrayLibrary.Array_Set` _best_lap_time _returnvalue 1.8647120722022892e+18 true)
        (`KismetArrayLibrary.Array_Set` _lap_start_time _returnvalue (`KismetSystemLibrary.GetGameTimeInSeconds`) true)
        (else
          (goto _label))))))

(event `self.ReceiveBeginPlay`
  (bind _asgm_default_race (cast `/Game/CustomPhysicVehicle/GM_Default_Race` (`GameplayStatics.GetGameMode`))))

(fn `UserConstructionScript`)