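; Spline-driven fence actor for race track environments, built in the Construction Script.
; It splits the spline into NumberOfMeshes equal-length spline mesh segments, setting tangents and roll from the spline, with end tangents zeroed.
; AdaptFenceToTerrain is a self-resetting toggle that, after segments are built, line-traces vertically to move every spline point except the last onto hit geometry.
; Track Start-End and Track Roll helpers compute per-point segment data but are not called here.
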(fn `Track Roll`
  (params (PointIndex :type Integer))
  (returns (`Start Roll` :type "Float (double-precision)") (`End Roll` :type "Float (double-precision)") (`Any Roll?` :type Boolean))
  (bind _spline (`self.Spline`))
  (bind _returnvalue (`SplineComponent.GetRollAtSplinePoint` _spline (+ PointIndex 1) "Local"))
  (bind _returnvalue_2 (`SplineComponent.GetRollAtSplinePoint` _spline PointIndex "Local"))
  (return (/ _returnvalue_2 25.0) (/ _returnvalue 25.0) (or (> (`KismetMathLibrary.Abs` _returnvalue_2) 1.0) (> (`KismetMathLibrary.Abs` _returnvalue) 1.0))))

(fn `Track Start-End`
  (params (`Lateral Offset` :type "Float (double-precision)") (PointIndex :type Integer))
  (returns (`Start Tangent` :type "Vector Structure") (`Start Location` :type "Vector Structure") (`End Tangent` :type "Vector Structure") (`End Location` :type "Vector Structure"))
  (bind _returnvalue (+ PointIndex 1))
  (bind _spline (`self.Spline`))
  (bind (_returnvalue_location _returnvalue_rotation) (`KismetMathLibrary.BreakTransform` (`SplineComponent.GetTransformAtSplinePoint` _spline PointIndex "Local" false)))
  (bind _returnvalue_2 (`KismetMathLibrary.SelectInt` _returnvalue (`KismetMathLibrary.SelectInt` 0 PointIndex) (<= _returnvalue (- (`SplineComponent.GetNumberOfSplinePoints` (`self.Spline`)) 1))))
  (bind (_returnvalue_location_2 _returnvalue_rotation_2) (`KismetMathLibrary.BreakTransform` (`SplineComponent.GetTransformAtSplinePoint` _spline _returnvalue_2 "Local" false)))
  (return (`SplineComponent.GetTangentAtSplinePoint` _spline PointIndex "Local") (+ (+ _returnvalue_location (* (`KismetMathLibrary.GetRightVector` _returnvalue_rotation) `Lateral Offset`)) (0.0 0.0 0.0)) (`SplineComponent.GetTangentAtSplinePoint` _spline _returnvalue_2 "Local") (+ (+ _returnvalue_location_2 (* (`KismetMathLibrary.GetRightVector` _returnvalue_rotation_2) `Lateral Offset`)) (0.0 0.0 0.0))))

(fn `UserConstructionScript`
  (bind _spline (`self.Spline`))
  (bind _returnvalue (* (`self.Index`) (`self.Length per Mesh`)))
  (bind _returnvalue_2 (- (`SplineComponent.GetNumberOfSplinePoints` _spline) 1))
  (bind _returnvalue_3 (* (+ (`self.Index`) 1) (`self.Length per Mesh`)))
  (set `self.Length per Mesh` (/ (`SplineComponent.GetSplineLength` (`self.Spline`)) (`KismetMathLibrary.Conv_IntToDouble` (`self.Number of Meshes`))))
  (for _index (range (`self.Number of Meshes`))
    (set `self.Index` _index)
    (bind _returnvalue_4 (`AddComponent|NODE_AddSplineMeshComponent-7`))
    (`SplineMeshComponent.SetStartAndEnd` _returnvalue_4 (`SplineComponent.GetLocationAtDistanceAlongSpline` (`self.Spline`) _returnvalue "Local") (* (`KismetMathLibrary.Normal` (`SplineComponent.GetTangentAtDistanceAlongSpline` (`self.Spline`) _returnvalue "Local")) (`self.Length per Mesh`)) (`SplineComponent.GetLocationAtDistanceAlongSpline` (`self.Spline`) _returnvalue_3 "Local") (* (`KismetMathLibrary.Normal` (`SplineComponent.GetTangentAtDistanceAlongSpline` (`self.Spline`) _returnvalue_3 "Local")) 0.0) true)
    (`SplineMeshComponent.SetStartRoll` _returnvalue_4 (/ (`SplineComponent.GetRollAtDistanceAlongSpline` (`self.Spline`) (* (`self.Index`) (`self.Length per Mesh`)) "Local") 90.0) true)
    (`SplineMeshComponent.SetEndRoll` _returnvalue_4 (/ (`SplineComponent.GetRollAtDistanceAlongSpline` (`self.Spline`) (* (+ (`self.Index`) 1) (`self.Length per Mesh`)) "Local") 90.0) true))
  (if (`self.Adapt Fence to Terrain`)
    (set `self.Adapt Fence to Terrain` false)
    (for _index_2 (range (+ _returnvalue_2 1))
      (if (not (== _index_2 _returnvalue_2))
        (bind _returnvalue_5 (`SplineComponent.GetLocationAtSplinePoint` _spline _index_2 "World"))
        (bind _outhit (`KismetSystemLibrary.LineTraceSingleForObjects` (+ _returnvalue_5 (0.0 0.0 50000.0)) (+ _returnvalue_5 (0.0 0.0 -50000.0)) (`|MakeArray` "ObjectTypeQuery1" "ObjectTypeQuery2" :!type "EObjectTypeQuery Enum")))
        (`SplineComponent.SetLocationAtSplinePoint` _spline _index_2 (`.Location` (`GameplayStatics.BreakHitResult` _outhit)) "World" true)))))