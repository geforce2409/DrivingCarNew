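; Game mode that spawns the player's selected car when play begins and hands it to the first player controller.
; It reads the car class from BP_GameInstance, spawns it at a Player Start with exiting and camera auto-rotation turned off, then possesses it.
; It finally calls DisableInput on every BP_Master_Vehicle in the level, with no exception made for the spawned car.
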(event `self.ReceiveBeginPlay`
  (bind _asbp_game_instance (cast `/Game/CustomPhysicVehicle/BP_GameInstance` (`GameplayStatics.GetGameInstance`)))
  (bind _returnvalue (`|SpawnActorFromClass` (`/Game/CustomPhysicVehicle/BP_GameInstance.Selected Car` _asbp_game_instance) (`self.GetTransform` (`self.K2_FindPlayerStart` null)) "AdjustIfPossibleButAlwaysSpawn" "OverrideRootScale" null false true true true true true true false false false false false false 1.0 1.5 0.0 "/Game/CustomPhysicVehicle/Vehicles/00_Master_Vehicle/Materials/M_default.M_default" null true null))
  (set `/Game/CustomPhysicVehicle/Vehicles/00_Master_Vehicle/BP_Master_Vehicle.Auto Rotate Camera` false _returnvalue)
  (`Controller.Possess` (`GameplayStatics.GetPlayerController` 0) _returnvalue)
  (bind _outactors (`GameplayStatics.GetAllActorsOfClass` "/Game/CustomPhysicVehicle/Vehicles/00_Master_Vehicle/BP_Master_Vehicle.BP_Master_Vehicle_C"))
  (for _array_element _outactors
    (`self.DisableInput` _array_element null)))

(fn `UserConstructionScript`)